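; BP_ShowShopTrigger is a trigger actor that toggles the ItemShop game feature when a player walks into its Box.
; On Box begin overlap, any overlapping Pawn has its movement stopped immediately, before the PlayerController check.
; For player-controlled pawns, it asks BSGameFeatureSystem whether ItemShop is active, then disables or enables it, so each new entry flips the state.
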(event `self.Box.OnComponentBeginOverlap`
  (params (OverlappedComponent :type "PrimitiveComponent Object Reference") (OtherActor :type "Actor Object Reference") (OtherComp :type "PrimitiveComponent Object Reference") (OtherBodyIndex :type Integer) (bFromSweep :type Boolean) (SweepResult :type "HitResult Structure (by ref)"))
  (bind _returnvalue (subsystem `BSGameFeatureSystem`))
  (bind `_as폰` (cast `Pawn` OtherActor))
  (`MovementComponent.StopMovementImmediately` (`Pawn.GetMovementComponent` `_as폰`))
  (cast `PlayerController` (`Pawn.GetController` `_as폰`))
  (bind _returnvalue_2 (`BSGameFeatureSystem.K2_IsGameFeatureActive` (subsystem `BSGameFeatureSystem`) "ItemShop"))
  (if _returnvalue_2
    (`BSGameFeatureSystem.K2_DisableGameFeature` _returnvalue "ItemShop")
    (else
      (`BSGameFeatureSystem.K2_EnableGameFeature` _returnvalue "ItemShop"))))

(fn `UserConstructionScript`)